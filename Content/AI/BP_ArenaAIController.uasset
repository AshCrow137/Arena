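; BP_ArenaAIController is the AI controller for arena characters, driven by the BT_ArenaCharacter behavior tree.
; On BeginPlay it starts the tree and writes the first player character's current position to the Location1 blackboard key.
; After a five-second delay it writes that player's new position to Location2, so both keys are one-time snapshots rather than continuously tracked targets.
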(event `self.ReceiveBeginPlay`
  (`self.RunBehaviorTree` "/Game/AI/BT_ArenaCharacter.BT_ArenaCharacter")
  (`BlackboardComponent.SetValueAsVector` (`AIBlueprintHelperLibrary.GetBlackboard` null) "Location1" (`self.K2_GetActorLocation` (`GameplayStatics.GetPlayerCharacter` 0)))
  (`KismetSystemLibrary.Delay` 5.0)
  (`BlackboardComponent.SetValueAsVector` (`AIBlueprintHelperLibrary.GetBlackboard` null) "Location2" (`self.K2_GetActorLocation` (`GameplayStatics.GetPlayerCharacter` 0))))

(fn `UserConstructionScript`)