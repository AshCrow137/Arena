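; Game instance for an arena match that keeps the player and AI scores across level reloads.
; SetupScore pushes both scores to the BP_HUD score widget, retrying each tick through a zero Delay loop until that widget is valid.
; UpPlayerScore and UpAIScore increment their score, update the widget, then reopen ThirdPersonExampleMap to start the next round.
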(event `SetupScore`
  (bind _asbp_hud (cast `/Game/Widgets/BP_HUD` (`PlayerController.GetHUD` (`GameplayStatics.GetPlayerController` 0))))
  (bind _userscorewidget (`/Game/Widgets/BP_HUD.UserScoreWidget` _asbp_hud))
  (`/Engine/EditorBlueprintResources/StandardMacros.IsValid` _userscorewidget :!label _label
    (:`Is Valid`
      (`/Game/Widgets/BP_UserScore.UpdatePlayer1Score` _userscorewidget (`self.PlayerOneScore`))
      (`/Game/Widgets/BP_UserScore.UpdatePlayer2Score` _userscorewidget (`self.PlayerTwoScore`)))
    (:`Is Not Valid`
      (`KismetSystemLibrary.Delay` 0.0)
      (goto _label))))

(event `self.UpPlayerScore`
  (bind _result (`/Engine/EditorBlueprintResources/StandardMacros.IncrementInt` (`self.PlayerOneScore`))
    (:`  `
      (bind _asbp_hud (cast `/Game/Widgets/BP_HUD` (`PlayerController.GetHUD` (`GameplayStatics.GetPlayerController` 0))))
      (`/Game/Widgets/BP_UserScore.UpdatePlayer1Score` (`/Game/Widgets/BP_HUD.UserScoreWidget` _asbp_hud) _result)
      (`GameplayStatics.OpenLevelBySoftObjectPtr` "/Game/ThirdPersonCPP/Maps/ThirdPersonExampleMap.ThirdPersonExampleMap"))))

(event `self.UpAIScore`
  (bind _result (`/Engine/EditorBlueprintResources/StandardMacros.IncrementInt` (`self.PlayerTwoScore`))
    (:`  `
      (bind _asbp_hud (cast `/Game/Widgets/BP_HUD` (`PlayerController.GetHUD` (`GameplayStatics.GetPlayerController` 0))))
      (`/Game/Widgets/BP_UserScore.UpdatePlayer2Score` (`/Game/Widgets/BP_HUD.UserScoreWidget` _asbp_hud) _result)
      (`GameplayStatics.OpenLevelBySoftObjectPtr` "/Game/ThirdPersonCPP/Maps/ThirdPersonExampleMap.ThirdPersonExampleMap"))))